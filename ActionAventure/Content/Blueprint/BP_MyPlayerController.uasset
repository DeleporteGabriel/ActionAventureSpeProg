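; Player controller that holds the player's health, mana, gold and spell list, and creates the main HUD and a shield effect widget.
; Stat functions update values and push them to the HUD, with damage starting a retriggerable invincibility window whose end removes the shield widget.
; A Shrinking event temporarily rescales the character.
; Keys cast or cycle spells, passing the controller and character to the spell, or directly trigger stat changes.
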(event `self.ReceiveBeginPlay`
  (`|ExecutionSequence`
    (:`then_0`
      (bind _returnvalue (`|CreateWidget` "/Game/Blueprint/WBP_InterfacePrincipale.WBP_InterfacePrincipale_C"))
      (bind _output_get (set `self.MainInterface` _returnvalue))
      (`UserWidget.AddToViewport` _output_get 0))
    (:`then_1`
      (bind _returnvalue_2 (`|CreateWidget` "/Game/Blueprint/WBP_ShieldEffect.WBP_ShieldEffect_C"))
      (set `self.ShieldUI` _returnvalue_2))
    (:`then_2`
      (set `self.PV` (`self.MaxPV`))
      (set `self.Mana` (`self.MaxMana`)))
    (:`then_3`
      (bind _asthird_person_character (cast `/Game/ThirdPersonBP/Blueprints/ThirdPersonCharacter` (`GameplayStatics.GetPlayerPawn` 0)))
      (set `self.ThirdPersonCharacter` _asthird_person_character))))

(event `Key|E`
  (params (Key :type "Key Structure"))
  (:`Pressed`
    (`self.DamageTaken` 10)))

(event `Key|A`
  (params (Key :type "Key Structure"))
  (:`Pressed`
    (`self.ManaUsed` 10)))

(event `Invincibility`
  (params (Duration :type "Float (double-precision)"))
  (set `self.InvincibilityFrame` true)
  (`KismetSystemLibrary.RetriggerableDelay` Duration)
  (set `self.InvincibilityFrame` false)
  (`Widget.RemoveFromParent` (`self.ShieldUI`)))

(event `Key|R`
  (params (Key :type "Key Structure"))
  (:`Pressed`
    (`self.GoldSpent` 10)))

(event `Shrinking`
  (params (Duration :type "Float (double-precision)") (NewScale3D :type "Vector Structure"))
  (`self.SetActorScale3D` (`self.ThirdPersonCharacter`) NewScale3D)
  (`KismetSystemLibrary.RetriggerableDelay` Duration)
  (`self.SetActorScale3D` (`self.ThirdPersonCharacter`) (1.0 1.0 1.0)))

(event `Key|T`
  (params (Key :type "Key Structure"))
  (:`Pressed`
    (`self.GoldGained` 30)))

(event `Key|M`
  (params (Key :type "Key Structure"))
  (:`Pressed`
    (`/Game/Blueprint/BP_DA_Spell.IsUsed` (`|GetArrayItem` (`self.SpellList`) (`self.CurrentSpell`)) self (`self.ThirdPersonCharacter`))))

(event `Key|I`
  (params (Key :type "Key Structure"))
  (:`Pressed`
    (`|ExecutionSequence`
      (:`then_0`
        (bind _output_get (set `self.CurrentSpell` (+ (`self.CurrentSpell`) 1)))
        (if (>= _output_get (`KismetArrayLibrary.Array_Length` (`self.SpellList`)))
          (set `self.CurrentSpell` 0)))
      (:`then_1`
        (`/Game/Blueprint/WBP_InterfacePrincipale.EditSpellIcon` (`self.MainInterface`) (`/Game/Blueprint/BP_DA_Spell.Icon` (`|GetArrayItem` (`self.SpellList`) (`self.CurrentSpell`))))))))

(fn `DamageHealed`
  (params (Healing :type Integer))
  (bind _output_get (set `self.PV` (`KismetMathLibrary.Clamp` (+ (`self.PV`) Healing) 0 (`self.MaxPV`))))
  (`/Game/Blueprint/WBP_InterfacePrincipale.EditPV` (`self.MainInterface`) (/ (`KismetMathLibrary.Conv_IntToDouble` _output_get) (`KismetMathLibrary.Conv_IntToDouble` (`self.MaxPV`)))))

(fn `DamageTaken`
  (params (Damage :type Integer))
  (if (not (`self.InvincibilityFrame`))
    (bind _output_get (set `self.PV` (`KismetMathLibrary.Clamp` (- (`self.PV`) Damage) 0 (`self.MaxPV`))))
    (`/Game/Blueprint/WBP_InterfacePrincipale.EditPV` (`self.MainInterface`) (/ (`KismetMathLibrary.Conv_IntToDouble` _output_get) (`KismetMathLibrary.Conv_IntToDouble` (`self.MaxPV`))))
    (`self.Invincibility` (`self.InvincibilityDuration`))))

(fn `GoldGained`
  (params (GoldAmount :type Integer))
  (bind _output_get (set `self.Gold` (+ (`self.Gold`) GoldAmount)))
  (`/Game/Blueprint/WBP_InterfacePrincipale.EditGold` (`self.MainInterface`) _output_get))

(fn `GoldSpent`
  (params (AmountSpent :type Integer))
  (if (>= (`self.Gold`) AmountSpent)
    (bind _output_get (set `self.Gold` (- (`self.Gold`) AmountSpent)))
    (`/Game/Blueprint/WBP_InterfacePrincipale.EditGold` (`self.MainInterface`) _output_get)))

(fn `ManaUsed`
  (params (ManaAmount :type Integer))
  (bind _output_get (set `self.Mana` (`KismetMathLibrary.Clamp` (- (`self.Mana`) ManaAmount) 0 (`self.MaxMana`))))
  (`/Game/Blueprint/WBP_InterfacePrincipale.EditMana` (`self.MainInterface`) (/ (`KismetMathLibrary.Conv_IntToDouble` _output_get) (`KismetMathLibrary.Conv_IntToDouble` (`self.MaxMana`)))))

(fn `UserConstructionScript`)