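; BP_SpellGiver is a purchasable spell pickup that sells MySpell to a player for GoldAmount in gold.
; The construction script shows the price on a text render and the spell's icon on a paper sprite.
; CoolEffect takes a controller, checks it can afford and lacks the spell, then deducts gold, adds the spell, refreshes its icon and prints a message.
; The event graph is empty, so CoolEffect relies on an external caller.
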(fn `CoolEffect`
  (params (Controler :type "/Game/Blueprint/BP_MyPlayerController Object Reference"))
  (bind _spelllist (`/Game/Blueprint/BP_MyPlayerController.SpellList` Controler))
  (if (>= (`/Game/Blueprint/BP_MyPlayerController.Gold` Controler) (`self.Gold Amount`))
    (if (== (`KismetArrayLibrary.Array_Find` _spelllist (`self.MySpell`)) -1)
      (`/Game/Blueprint/BP_MyPlayerController.GoldSpent` Controler (`self.Gold Amount`))
      (`KismetArrayLibrary.Array_Add` _spelllist (`self.MySpell`))
      (`/Game/Blueprint/BP_MyPlayerController.Update Spell Icon` Controler)
      (`KismetSystemLibrary.PrintString` (`KismetStringLibrary.Concat_StrStr` "You obtained the " (`/Game/Blueprint/BP_DA_Spell.Name` (`self.MySpell`)) " spell !")))))

(fn `UserConstructionScript`
  (`TextRenderComponent.K2_SetText` (`self.TextRender`) (`KismetTextLibrary.Conv_StringToText` (`KismetStringLibrary.Concat_StrStr` (`KismetStringLibrary.Conv_IntToString` (`self.Gold Amount`)) " GOLDS")))
  (`PaperSpriteComponent.SetSprite` (`self.PaperSprite`) (`/Game/Blueprint/BP_DA_Spell.Icon` (`self.MySpell`))))